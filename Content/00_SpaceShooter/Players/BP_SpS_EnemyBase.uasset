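; Base enemy ship for the space shooter that flies in a straight line along its starting forward vector and fires missiles from its fire point on a timer.
; Overlapping an actor tagged "Bottom" silently removes it, while a friendly missile fires its kill dispatcher and notifies BP_GameMode.
; The bound kill handler rolls a drop chance to play a sound and spawn a random-type item, then destroys the enemy after a brief delay.
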(event `self.ReceiveActorBeginOverlap`
  (params (OtherActor :type "Actor Object Reference"))
  (if (`KismetArrayLibrary.Array_Contains` (`Actor.Tags` OtherActor) "Bottom")
    (`self.K2_DestroyActor`)
    (else
      (bind _asbp_sp_s_missile (cast `/Game/00_SpaceShooter/Players/BP_SpS_Missile` OtherActor))
      (if (`/Game/00_SpaceShooter/Players/BP_SpS_Missile.IsFriendly` _asbp_sp_s_missile)
        (`self.OnEnemyKill`)
        (bind _asbp_game_mode (cast `/Game/00_SpaceShooter/BP_GameMode` (`GameplayStatics.GetGameMode`)))
        (`/Game/00_SpaceShooter/BP_GameMode.OnEnemyKill` _asbp_game_mode)))))

(event `self.ReceiveBeginPlay`
  (set `self.MovementVector` (`self.GetActorForwardVector`))
  (add `self.OnEnemyKill` (delegate `Kill Event`)))

(event `Kill Event`
  (`self.F_SpawnItem`)
  (`KismetSystemLibrary.Delay` 0.1)
  (`self.K2_DestroyActor`))

(event `self.ReceiveTick`
  (params (DeltaSeconds :type "Float (single-precision)"))
  (`self.F_Move` DeltaSeconds)
  (bind _output_get (set `self.ShotCurentTime` (+ DeltaSeconds (`self.ShotCurentTime`))))
  (if (> _output_get (`self.DelayShot`))
    (set `self.ShotCurentTime` 0.0)
    (`self.F_SpawnMissile` 600.0)))

(fn `F_Move`
  (params (A :type "Float (double-precision)"))
  (`self.K2_SetActorLocation` (+ (`self.K2_GetActorLocation`) (* (* A (`self.Speed`)) (`self.MovementVector`)))))

(fn `F_SpawnItem`
  (if (<= (`KismetMathLibrary.RandomFloatInRange` 0.0 1.0) (`self.DropChance`))
    (`GameplayStatics.PlaySound2D` "/Engine/EditorSounds/GamePreview/EndSimulate.EndSimulate" 1.0 1.0 0.0 null null)
    (`|SpawnActorFromClass` "/Game/00_SpaceShooter/BP_Item.BP_Item_C" (`SceneComponent.K2_GetComponentToWorld` (`self.Capsule`)) "Undefined" "MultiplyWithRoot" null (cast `/Game/00_SpaceShooter/E_ItemType` (`KismetMathLibrary.Conv_IntToByte` (`KismetMathLibrary.RandomIntegerInRange` 0 (- (enumcount `/Game/00_SpaceShooter/E_ItemType`) 1)))) null)))

(fn `F_SpawnMissile`
  (params (Speed :type "Float (double-precision)"))
  (bind _firepoint (`self.FirePoint`))
  (`/Engine/EditorBlueprintResources/StandardMacros.IsValid` _firepoint
    (:`Is Valid`
      (bind _returnvalue (`|SpawnActorFromClass` "/Game/00_SpaceShooter/Players/BP_SpS_Missile.BP_SpS_Missile_C" (`SceneComponent.K2_GetComponentToWorld` _firepoint) "Undefined" "MultiplyWithRoot" null Speed false -25.0 null))
      (`/Engine/EditorBlueprintResources/StandardMacros.IsValid` _returnvalue
        (:`Is Valid`
          (`self.K2_SetActorRotation` _returnvalue (`self.K2_GetActorRotation`) false))))))

(fn `UserConstructionScript`)