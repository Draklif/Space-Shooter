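; BP_SpS_EnemyTurret is an enemy turret in the space shooter that turns to track the player.
; On BeginPlay it caches the player pawn as a BP_SpS_Player reference.
; Each Tick it interpolates toward the look-at rotation at RotationSpeed and applies only the yaw, so it swivels horizontally.
; Parent events are called first, and this graph contains no firing logic of its own.
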(event `self.ReceiveBeginPlay`
  (`parent.ReceiveBeginPlay`)
  (bind _asbp_sp_s_player (cast `/Game/00_SpaceShooter/Players/BP_SpS_Player` (`GameplayStatics.GetPlayerPawn` 0)))
  (set `self.Player Ref` _asbp_sp_s_player))

(event `self.ReceiveTick`
  (params (DeltaSeconds :type "Float (single-precision)"))
  (bind (_returnvalue_roll _returnvalue_pitch _returnvalue_yaw) (`KismetMathLibrary.BreakRotator` (`KismetMathLibrary.RInterpTo` (`self.K2_GetActorRotation`) (`KismetMathLibrary.FindLookAtRotation` (`self.K2_GetActorLocation`) (`self.K2_GetActorLocation` (`self.Player Ref`))) (`GameplayStatics.GetWorldDeltaSeconds`) (`self.Rotation Speed`))))
  (`parent.ReceiveTick` DeltaSeconds)
  (`self.K2_SetActorRotation` (`KismetMathLibrary.MakeRotator` 0.0 0.0 _returnvalue_yaw)))

(fn `UserConstructionScript`
  (`parent.UserConstructionScript`))