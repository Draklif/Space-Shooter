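; Player ship for the space shooter, handling Enhanced Input movement with per-wing lateral scaling, weapons, health and death.
; Single and recursive burst shots spawn friendly missiles behind a fire-rate timer, while the timed laser pickup skips the cooldown.
; Overlaps apply enemy collisions, hostile missile damage and item pickups.
; Zero HP fires a death event that explodes the ship and opens the game-over widget; Tick accumulates elapsed time as distance.
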(event `Death Event`
  (bind _capsulecomponent (`self.CapsuleComponent`))
  (`GameplayStatics.SpawnEmitterAtLocation` "/Game/StarterContent/Particles/P_Explosion.P_Explosion" (`self.K2_GetActorLocation`) (struct) (2.0 2.0 2.0))
  (`SceneComponent.SetVisibility` (`self.SM_StarSparrow01`) false false)
  (`KismetSystemLibrary.Delay` 0.2)
  (`/Engine/EditorBlueprintResources/StandardMacros.IsValid` _capsulecomponent
    (:`Is Valid`
      (`ActorComponent.K2_DestroyComponent` _capsulecomponent)
      (`KismetSystemLibrary.Delay` 1.0)
      (bind _returnvalue (`|CreateWidget` "/Game/00_SpaceShooter/WBP_GameOver.WBP_GameOver_C"))
      (`/Game/00_SpaceShooter/WBP_GameOver.Enable Key Press` _returnvalue)
      (`UserWidget.AddToViewport` _returnvalue 0))))

(event `self.ReceiveBeginPlay`
  (bind _asplayer_controller (cast `PlayerController` (`self.GetController`)))
  (bind _returnvalue (pcsubsystem `EnhancedInputLocalPlayerSubsystem` _asplayer_controller))
  (`/Engine/EditorBlueprintResources/StandardMacros.IsValid` _returnvalue
    (:`Is Valid`
      (`EnhancedInputSubsystemInterface.AddMappingContext` _returnvalue "/Game/00_SpaceShooter/Input/IMC_PC.IMC_PC" 0 (struct))
      (add `self.OnPlayerDeath` (delegate `Death Event`)))))

(event `self.ReceiveTick`
  (params (DeltaSeconds :type "Float (single-precision)"))
  (set `self.CurrentDistance` (+ DeltaSeconds (`self.CurrentDistance`))))

(event `EnhancedInput|/Game/00_SpaceShooter/Input/IA_Move`
  (params (ActionValue :type "Vector2D Structure") (ElapsedSeconds :type "Float (double-precision)") (TriggeredSeconds :type "Float (double-precision)") (InputAction :type "InputAction Object Reference" :default "/Game/00_SpaceShooter/Input/IA_Move.IA_Move"))
  (bind _returnvalue (`self.GetActorRightVector`))
  (:`Triggered`
    (if (> ActionValue_X 0.0)
      (`self.AddMovementInput` _returnvalue (* ActionValue_X (`self.RightWing`)))
      (else
        (`self.AddMovementInput` _returnvalue (* ActionValue_X (`self.LeftWing`)))))
    (`self.AddMovementInput` (`self.GetActorForwardVector`) ActionValue_Y)))

(event `self.ReceiveActorBeginOverlap`
  (params (OtherActor :type "Actor Object Reference"))
  (cast `/Game/00_SpaceShooter/Players/BP_SpS_EnemyBase` OtherActor
    (:`then`
      (`self.F_ModifyHP` -1000.0)
      (`GameplayStatics.PlaySound2D` "/Game/StarterContent/Audio/Explosion_Cue.Explosion_Cue" 1.0 1.0 0.0 null null))
    (:`CastFailed`
      (bind _asbp_sp_s_missile (cast `/Game/00_SpaceShooter/Players/BP_SpS_Missile` OtherActor)
        (:`then`
          (if (not (`/Game/00_SpaceShooter/Players/BP_SpS_Missile.IsFriendly` _asbp_sp_s_missile))
            (`self.F_ModifyHP` (`/Game/00_SpaceShooter/Players/BP_SpS_Missile.Damage` _asbp_sp_s_missile))
            (`self.K2_DestroyActor` _asbp_sp_s_missile)))
        (:`CastFailed`
          (bind _asbp_item (cast `/Game/00_SpaceShooter/BP_Item` OtherActor))
          (`GameplayStatics.PlaySound2D` "/Engine/VREditor/Sounds/UI/Dockable_Window_Drop.Dockable_Window_Drop" 1.0 1.0 0.0 null null)
          (switch `/Game/00_SpaceShooter/E_ItemType` (`/Game/00_SpaceShooter/BP_Item.ItemType` _asbp_item)
            (:`NewEnumerator0`
              (`self.F_ModifyHP` 25.0))
            (:`NewEnumerator1`
              (`self.F_ModifyFireRate` -0.1))
            (:`NewEnumerator2`
              (set `self.CurrentWeapon` "NewEnumerator1"))
            (:`NewEnumerator3`
              (set `self.CurrentWeapon` "NewEnumerator0"))
            (:`NewEnumerator4`
              (set `self.CurrentWeapon` "NewEnumerator2")
              (`KismetSystemLibrary.K2_SetTimerDelegate` (delegate `LaserOff`) 10.0)
              (`GameplayStatics.PlaySound2D` "/Engine/VREditor/Sounds/VR_teleport.VR_teleport" 0.5 1.0 0.0 null null))))))))

(event `EnhancedInput|/Game/00_SpaceShooter/Input/IA_Fire`
  (params (ActionValue :type Boolean) (ElapsedSeconds :type "Float (double-precision)") (TriggeredSeconds :type "Float (double-precision)") (InputAction :type "InputAction Object Reference" :default "/Game/00_SpaceShooter/Input/IA_Fire.IA_Fire"))
  (:`Triggered`
    (if (`self.CanFire`)
      (switch `/Game/00_SpaceShooter/E_WeaponType` (`self.CurrentWeapon`)
        (:`NewEnumerator0`
          (`self.Single Shot`))
        (:`NewEnumerator1`
          (`self.Burst Shot`))
        (:`NewEnumerator2`
          (`self.F_SpawnMissile` 1500.0))))))

(event `EnhancedInput|/Game/00_SpaceShooter/Input/IA_Quit`
  (params (ActionValue :type "Vector2D Structure") (ElapsedSeconds :type "Float (double-precision)") (TriggeredSeconds :type "Float (double-precision)") (InputAction :type "InputAction Object Reference" :default "/Game/00_SpaceShooter/Input/IA_Quit.IA_Quit"))
  (:`Triggered`
    (`KismetSystemLibrary.QuitGame` null "Quit")))

(event `Single Shot`
  (`self.F_SpawnMissile` 1000.0)
  (set `self.CanFire` false)
  (bind _returnvalue (`KismetSystemLibrary.K2_SetTimerDelegate` (delegate `UpdateCanShoot`) (`self.FireRate`)))
  (set `self.FireCooldown` _returnvalue))

(event `LaserOff`
  (if (`|EnumEquality` (`self.CurrentWeapon`) "NewEnumerator2")
    (set `self.CurrentWeapon` "NewEnumerator0")))

(event `Burst Shot`
  (if (> (`self.BurstCount_Current`) 0)
    (`self.F_SpawnMissile` 1000.0)
    (set `self.CanFire` false)
    (`/Engine/EditorBlueprintResources/StandardMacros.DecrementInt` (`self.BurstCount_Current`)
      (:`  `
        (`KismetSystemLibrary.Delay` 0.05)
        (`self.Burst Shot`)))
    (else
      (`KismetSystemLibrary.Delay` 0.2)
      (set `self.BurstCount_Current` (`self.BurstCount_Default`))
      (bind _returnvalue (`KismetSystemLibrary.K2_SetTimerDelegate` (delegate `UpdateCanShoot`) (`self.FireRate`)))
      (set `self.FireCooldown` _returnvalue))))

(event `UpdateCanShoot`
  (set `self.CanFire` true))

(fn `F_ModifyFireRate`
  (params (Value :type "Float (double-precision)"))
  (set `self.FireRate` (`KismetMathLibrary.FClamp` (+ (`self.FireRate`) Value) 0.1 2.0)))

(fn `F_ModifyHP`
  (params (Value :type "Float (double-precision)"))
  (bind _output_get (set `self.HP` (`KismetMathLibrary.FClamp` (+ (`self.HP`) Value) 0.0 (`self.HP_Max`))))
  (if (<= _output_get 0.0)
    (`self.OnPlayerDeath`)))

(fn `F_SpawnMissile`
  (params (Speed :type "Float (double-precision)"))
  (`|SpawnActorFromClass` "/Game/00_SpaceShooter/Players/BP_SpS_Missile.BP_SpS_Missile_C" (`SceneComponent.K2_GetComponentToWorld` (`self.FirePoint`)) "Undefined" "MultiplyWithRoot" self Speed true -25.0 null))

(fn `UserConstructionScript`)