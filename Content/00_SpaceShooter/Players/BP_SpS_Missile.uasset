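; BP_SpS_Missile is a space shooter projectile that flies straight along its forward vector and expires after a short lifespan.
; Tick moves it by Speed and delta time without sweeping.
; On overlap, IsFriendly and actor tags filter out its own side, bullets, walls and items, then a DoOnce plays the explosion particle and sound.
; The graph applies no damage and does not destroy the missile on impact.
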(event `self.ReceiveActorBeginOverlap`
  (params (OtherActor :type "Actor Object Reference"))
  (if (and (`self.IsFriendly`) (`self.ActorHasTag` OtherActor "Player"))
    _
    (elif (and (not (`self.IsFriendly`)) (`self.ActorHasTag` OtherActor "Enemy"))
      _
      (elif (not (or (`self.ActorHasTag` OtherActor "Bullet") (`self.ActorHasTag` OtherActor "Wall") (`self.ActorHasTag` OtherActor "Item")))
        (`/Engine/EditorBlueprintResources/StandardMacros.DoOnce` false
          (:`Completed`
            (`GameplayStatics.SpawnEmitterAtLocation` "/Game/StarterContent/Particles/P_Explosion.P_Explosion" (`self.K2_GetActorLocation`))
            (`GameplayStatics.PlaySound2D` "/Game/StarterContent/Audio/Explosion_Cue.Explosion_Cue" 1.0 1.0 0.0 null null)))))))

(event `self.ReceiveBeginPlay`
  (`self.SetLifeSpan` 5.0))

(event `self.ReceiveTick`
  (params (DeltaSeconds :type "Float (single-precision)"))
  (`self.K2_SetActorLocation` (+ (* (* DeltaSeconds (`self.Speed`)) (`self.GetActorForwardVector`)) (`self.K2_GetActorLocation`))))

(fn `UserConstructionScript`)