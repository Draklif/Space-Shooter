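; BP_Item is a space shooter item actor that drifts in a straight line, with an ItemType of health, fire rate or one of several weapon types.
; BeginPlay picks a StarSparrow part mesh for the type and caches the forward vector, which Tick uses with Speed to move it.
; Overlapping an actor tagged Player or Bottom destroys it after a short delay; no pickup effect is applied here.
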(event `self.ReceiveBeginPlay`
  (bind _staticmesh (`self.StaticMesh`))
  (set `self.MovementVector` (`self.GetActorForwardVector`))
  (switch `/Game/00_SpaceShooter/E_ItemType` (`self.ItemType`)
    (:`NewEnumerator0`
      (`StaticMeshComponent.SetStaticMesh` _staticmesh "/Game/StarSparrow/Meshes/Modules/SM_Parts_StarSparrow_Engine.SM_Parts_StarSparrow_Engine"))
    (:`NewEnumerator1`
      (`StaticMeshComponent.SetStaticMesh` _staticmesh "/Game/StarSparrow/Meshes/Modules/SM_Parts_StarSparrow_Wing_03.SM_Parts_StarSparrow_Wing_03"))
    (:`NewEnumerator2`
      (`StaticMeshComponent.SetStaticMesh` _staticmesh "/Game/StarSparrow/Meshes/Modules/SM_Parts_StarSparrow_Weapon.SM_Parts_StarSparrow_Weapon"))
    (:`NewEnumerator3`
      (`StaticMeshComponent.SetStaticMesh` _staticmesh "/Game/StarSparrow/Meshes/Modules/SM_Parts_StarSparrow_Wing_01.SM_Parts_StarSparrow_Wing_01"))
    (:`NewEnumerator4`
      (`StaticMeshComponent.SetStaticMesh` _staticmesh "/Game/StarSparrow/Meshes/Modules/SM_Parts_StarSparrow_Engine.SM_Parts_StarSparrow_Engine"))))

(event `self.ReceiveTick`
  (params (DeltaSeconds :type "Float (single-precision)"))
  (`self.K2_SetActorLocation` (+ (`self.K2_GetActorLocation`) (* (* DeltaSeconds (`self.Speed`)) (`self.MovementVector`)))))

(event `self.ReceiveActorBeginOverlap`
  (params (OtherActor :type "Actor Object Reference"))
  (bind _tags (`Actor.Tags` OtherActor))
  (if (or (`KismetArrayLibrary.Array_Contains` _tags "Bottom") (`KismetArrayLibrary.Array_Contains` _tags "Player"))
    (`KismetSystemLibrary.Delay` 0.1)
    (`self.K2_DestroyActor`)))

(fn `UserConstructionScript`)